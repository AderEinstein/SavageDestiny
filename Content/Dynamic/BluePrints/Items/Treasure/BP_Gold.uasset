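; BP_Gold is a gold treasure item that adds its own feedback on top of a parent class's overlap behavior.
; When an actor overlaps it, it runs the parent handler, zeroes its rotation constant, then after a short delay plays a coin spill sound at its location.
; The overlap does not filter by actor, and BeginPlay, Tick and construction add no logic of their own.
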(event `self.ReceiveActorBeginOverlap`
  (params (OtherActor :type "Actor Object Reference"))
  (`parent.ReceiveActorBeginOverlap` OtherActor)
  (set `self.RotationConstant` 0.0)
  (`KismetSystemLibrary.Delay` 0.2)
  (`GameplayStatics.PlaySoundAtLocation` "/Game/Dynamic/Audio/MetaSounds/SFX_CoinSpill.SFX_CoinSpill" (`self.K2_GetActorLocation`) (struct) 1.0 1.0 0.0 null null null null))

(fn `UserConstructionScript`
  (`parent.UserConstructionScript`))