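; Breakable barrels Blueprint built from four Chaos Geometry Collections, each paired with a capsule.
; When any collection breaks, its capsule stops blocking Pawns and the whole actor gets a short lifespan before removal.
; Only the first collection's break also plays a pot-break sound and calls SpawnTreasure, so the other three give no sound or loot here.
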(event `self.GeometryCollection.OnChaosBreakEvent`
  (params (BreakEvent :type "ChaosBreakEvent Structure (by ref)"))
  (`GameplayStatics.PlaySoundAtLocation` "/Game/Dynamic/Audio/MetaSounds/SFX_PotBreak.SFX_PotBreak" (`self.K2_GetActorLocation`) (struct) 1.0 1.0 0.0 null null null null)
  (`self.SpawnTreasure`)
  (`self.SetLifeSpan` 3.0)
  (`PrimitiveComponent.SetCollisionResponseToChannel` (`self.Capsule`) "ECC_Pawn" "ECR_Ignore"))

(event `self.GeometryCollection1.OnChaosBreakEvent`
  (params (BreakEvent :type "ChaosBreakEvent Structure (by ref)"))
  (`self.SetLifeSpan` 3.0)
  (`PrimitiveComponent.SetCollisionResponseToChannel` (`self.Capsule1`) "ECC_Pawn" "ECR_Ignore"))

(event `self.GeometryCollection2.OnChaosBreakEvent`
  (params (BreakEvent :type "ChaosBreakEvent Structure (by ref)"))
  (`self.SetLifeSpan` 3.0)
  (`PrimitiveComponent.SetCollisionResponseToChannel` (`self.Capsule2`) "ECC_Pawn" "ECR_Ignore"))

(event `self.GeometryCollection3.OnChaosBreakEvent`
  (params (BreakEvent :type "ChaosBreakEvent Structure (by ref)"))
  (`self.SetLifeSpan` 3.0)
  (`PrimitiveComponent.SetCollisionResponseToChannel` (`self.Capsule3`) "ECC_Pawn" "ECR_Ignore"))

(fn `UserConstructionScript`)